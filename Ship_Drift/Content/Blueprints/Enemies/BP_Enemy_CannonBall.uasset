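; BP_Enemy_CannonBall is an enemy cannonball projectile that damages and knocks back the player.
; Spawn stores damage, lifetime and speed and plays the cannon sound.
; Tick moves it unswept by Direction times Speed per frame, without delta-time scaling, and destroys it when its lifetime expires.
; Overlapping BP_Player applies damage through Health, adds a speed-scaled forward impulse if the player survives, then destroys the ball.
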(event OnComponentBeginOverlap(Collider)
  (params (OverlappedComponent :type Primitive%20Component%20Object%20Reference) (OtherActor :type Actor%20Object%20Reference) (OtherComp :type Primitive%20Component%20Object%20Reference) (OtherBodyIndex :type Integer) (bFromSweep :type Boolean) (SweepResult :type Hit%20Result%20Structure%20%28by%20ref%29))
  ;[0.15 0.15 0.15 0.5] Handle Player Collision
  (if (== (Utilities|GetClass OtherActor) "/Game/Blueprints/Player/BP_Player.BP_Player_C")
    (bind _asbp_player (Utilities|Casting|CastToBP_Player OtherActor))
    (Default|TakeDamage (Variables|/Game/Blueprints/Player/BP_Player.BP_Player_C|GetHealth _asbp_player) (Variables|Default|Getdamage))
    (if (Default|IsAlive (Variables|/Game/Blueprints/Player/BP_Player.BP_Player_C|GetHealth _asbp_player))
      (Physics|AddImpulse (Variables|/Script/Engine.Character|GetCharacterMovement _asbp_player) (* (Transformation|GetActorForwardVector) (Variables|Default|Getspeed) 1e+03) false)
      (Actor|DestroyActor)
      (else
        (Actor|DestroyActor)))))

(event Custom|Spawn
  (params (damage :type Float%20%28double-precision%29) (time :type Float%20%28double-precision%29) (speed :type Float%20%28double-precision%29))
  (Variables|Default|Setdamage damage)
  (Variables|Default|Settime_left_alive time)
  (Variables|Default|Setspeed speed)
  (Audio|PlaySoundatLocation "/Game/Sound/SoundCue/Player/Cannon/A_Cannon_Cue.A_Cannon_Cue" (Transformation|GetActorLocation) "0, 0, 0" 1.0 1.0 0.0 0 0 0 0))

(event EventTick
  (params (DeltaSeconds :type Float%20%28single-precision%29))
  (Transformation|AddActorWorldOffset (* (Variables|Default|Getdirection) (Variables|Default|Getspeed)))
  (Variables|Default|Settime_left_alive (- (Variables|Default|Gettime_left_alive) DeltaSeconds))
  (if (<= (Variables|Default|Gettime_left_alive) 0.0)
    (Actor|DestroyActor)))

(fn ConstructionScript)